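; Inventory component for the player character BP_Wilson that stores stackable item slots and handles pickup and dropping.
; A per-tick sphere trace around the player tracks the look-at actor, which the pickup input sends to its item data component before refreshing the grid UI.
; Adds fill stacks up to DT_ItemData limits, then empty slots.
; Transfers swap differing slots between inventories, and non-consumed removals spawn pickups; both broadcast inventory updates.
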(event `self.ReceiveBeginPlay`
  (`KismetArrayLibrary.Array_Resize` (`self.Content`) (`self.InventorySize`)))

(event `self.ReceiveTick`
  (params (DeltaSeconds :type "Float (single-precision)"))
  (`self.InteractionTrace`))

(event `EnhancedInput|/Game/MyContent/Input/IA_Pickup`
  (params (ActionValue :type Boolean) (ElapsedSeconds :type "Float (double-precision)") (TriggeredSeconds :type "Float (double-precision)") (InputAction :type "InputAction Object Reference" :default "/Game/MyContent/Input/IA_Pickup.IA_Pickup"))
  (:`Started`
    (bind _lookatactor (`self.LookAtActor` :!label _label)
      (:`then`
        (bind _returnvalue (`Actor.GetComponentByClass` _lookatactor "/Game/MyContent/InventorySystem/BP_ItemDataComponent.BP_ItemDataComponent_C"))
        (`/Engine/EditorBlueprintResources/StandardMacros.IsValid` _returnvalue
          (:`Is Valid`
            (message `/Game/MyContent/InventorySystem/BI_InteractInterface.InteractWith` _returnvalue (cast `/Game/MyContent/Characters/BP_Wilson` (`self.GetOwner`) :!pure true) (`/Game/MyContent/Blueprint/BP_Object_Pickable.Quantity` (cast `/Game/MyContent/Blueprint/BP_Object_Pickable` _lookatactor :!pure true)))
            (`/Game/MyContent/InventorySystem/UI/UI_InventoryGrid.DisplayInventory` (`/Game/MyContent/InventorySystem/UI/UI_PlayerMenu.UI_InventoryGrid` (`.Menu` (`/Game/MyContent/Characters/UI_PlayerHUD.Menu` (`/Game/MyContent/Characters/BP_Wilson.HUD` (cast `/Game/MyContent/Characters/BP_Wilson` (`self.GetOwner`) :!pure true))))) (`Actor.GetComponentByClass` (`GameplayStatics.GetPlayerCharacter` 0) "BP_InventorySystem_C"))
            (bind _returnvalue_2 (`AnimInstance.Montage_Play` (`SkeletalMeshComponent.GetAnimInstance` (`Character.Mesh` (cast `/Game/MyContent/Characters/BP_Wilson` (`GameplayStatics.GetPlayerPawn` 0) :!pure true))) "/Game/MyContent/Characters/Wilson/Animations/AnimMontage_Interact.AnimMontage_Interact" 1.0 "MontageLength" 0.0 true))
            (`KismetSystemLibrary.Delay` (- _returnvalue_2 0.1)))
          (:`Is Not Valid`
            (`Actor.SetOwner` _lookatactor (`Pawn.GetController` (cast `/Game/MyContent/Characters/BP_Wilson` (`self.GetOwner`) :!pure true))))))
      (:`else`))))

(event `Grab`
  (goto _label))

(event `Update`
  (`self.OnInventoryUpdate`))

(event `TRNSFR_SLTS`
  (params (SourceIndex :type Integer) (SourceInventory :type "/Game/MyContent/InventorySystem/BP_InventorySystem Object Reference") (DestinationIndex :type Integer))
  (`self.TransferSlots` SourceIndex SourceInventory DestinationIndex))

(event `DropItem`
  (params (ItemID :type Name) (Quantity :type Integer))
  (bind _returnvalue (`GameplayStatics.GetPlayerPawn` 0))
  (bind _returnvalue_2 (`|SpawnActorFromClass` (`.ItemClass_12_51D999594EB474740A56898525B05F98` (break `/Game/MyContent/InventorySystem/ST_ItemStruct` (`self.GetItemData` ItemID))) (`KismetMathLibrary.MakeTransform` (`Actor.K2_GetActorLocation` _returnvalue) (`Actor.K2_GetActorRotation` _returnvalue)) "Undefined" "MultiplyWithRoot" null null))
  (set `/Game/MyContent/Blueprint/BP_Object_Pickable.Quantity` Quantity (cast `/Game/MyContent/Blueprint/BP_Object_Pickable` _returnvalue_2 :!pure true)))

(event `RMV_INVTRY`
  (params (Index :type Integer) (IsConsumed :type Boolean) (`WholeStack?` :type Boolean) (Amount :type Integer))
  (`self.RemoveFromInventory` Index IsConsumed `WholeStack?` Amount))

(fn `AddToInventory`
  (params (ItemID :type Name) (Quantity :type Integer))
  (returns (Succ :type Boolean) (QuantityRemaining :type Integer))
  (locals (LocalQuantityRemaining :type Integer) (Local_HasFailed :type Boolean))
  (set `local.LocalQuantityRemaining` Quantity)
  (while (and (> (`local.LocalQuantityRemaining`) 0) (not (`local.Local_HasFailed`)))
    (bind (_index _foundslot) (`self.FindSlot` (`local.ItemID`)))
    (if _foundslot
      (`self.AddToStack` _index 1)
      (`/Engine/EditorBlueprintResources/StandardMacros.DecrementInt` (`local.LocalQuantityRemaining`))
      (elif (`self.AnyEmptySlot`)
        (bind _succ (`self.CreateNewStack` (`local.ItemID`) 1))
        (if _succ
          (`/Engine/EditorBlueprintResources/StandardMacros.DecrementInt` (`local.LocalQuantityRemaining`))
          (else
            (set `local.Local_HasFailed` true)))
        (else
          (set `local.Local_HasFailed` true)))))
  (return (not (`local.Local_HasFailed`)) (`local.LocalQuantityRemaining`)))

(fn `AddToStack`
  (params (Index :type Integer) (Quantity :type Integer))
  (bind (_output_itemid _output_quantity) (break `/Game/MyContent/InventorySystem/ST_SlotStruct` (`|GetArrayItem` (`self.Content`) Index)))
  (`KismetArrayLibrary.Array_Set` (`self.Content`) Index (make `/Game/MyContent/InventorySystem/ST_SlotStruct` _output_itemid (+ _output_quantity Quantity))))

(fn `AnyEmptySlot`
  (returns (HasEmptySlot :type Boolean) (EmptyIndex :type Integer))
  (for (_array_element _array_index) (`self.Content`)
    (if (== (`.Quantity_6_FC6623174BF0FDD05402C19C63719A2F` (break `/Game/MyContent/InventorySystem/ST_SlotStruct` _array_element)) 0)
      (return true _array_index)))
  (return false -1))

(fn `CreateNewStack`
  (params (ItemID :type Name) (Quantity :type Integer))
  (returns (Succ :type Boolean))
  (bind (_hasemptyslot _emptyindex) (`self.AnyEmptySlot`))
  (if _hasemptyslot
    (`KismetArrayLibrary.Array_Set` (`self.Content`) _emptyindex (make `/Game/MyContent/InventorySystem/ST_SlotStruct` ItemID Quantity))
    (return true)
    (else
      (return false))))

(fn `FindSlot`
  (params (ItemID :type Name))
  (returns (Index :type Integer) (FoundSlot :type Boolean) (Quantity :type Integer))
  (bind _itemid (`local.ItemID`))
  (for (_array_element _array_index) (`self.Content`)
    (bind (_itemid_2 _quantity) (break `/Game/MyContent/InventorySystem/ST_SlotStruct` _array_element))
    (if (== _itemid_2 _itemid)
      (if (< _quantity (`self.GetMaxStackSize` _itemid))
        (return _array_index true _quantity))))
  (return -1 false 0))

(fn `GetDropLocation`
  (returns (Location :type "Vector Structure"))
  (return (`Actor.K2_GetActorLocation` (`GameplayStatics.GetPlayerPawn` 0))))

(fn `GetItemData`
  (params (ItemID :type Name))
  (returns (Data :type "/Game/MyContent/InventorySystem/ST_ItemStruct Structure"))
  (bind _returnvalue (`|GetDataTableRow` "/Game/MyContent/InventorySystem/DT_ItemData.DT_ItemData" ItemID)
    (:`then`
      (return _returnvalue))))

(fn `GetMaxStackSize`
  (params (ItemID :type Name))
  (returns (StackSize :type Integer))
  (bind _returnvalue (`|GetDataTableRow` "/Game/MyContent/InventorySystem/DT_ItemData.DT_ItemData" ItemID)
    (:`then`
      (return (`.StackSize_15_9BEB1E854F1882D8A719F4A4706126C4` (break `/Game/MyContent/InventorySystem/ST_ItemStruct` _returnvalue))))
    (:`RowNotFound`
      (return -1))))

(fn `InteractionTrace`
  (bind _returnvalue (`Actor.K2_GetActorLocation` (`GameplayStatics.GetPlayerPawn` 0)))
  (bind (_outhit _returnvalue_2) (`KismetSystemLibrary.SphereTraceSingle` (+ _returnvalue (0.0 0.0 100.0)) (+ _returnvalue (0.0 0.0 -75.0)) 75.0 "TraceTypeQuery3" false (`|MakeArray` null :!type "Actor Object Reference")))
  (if _returnvalue_2
    (bind (_bblockinghit _binitialoverlap _time _distance _location _impactpoint _normal _impactnormal _physmat _hitactor) (`GameplayStatics.BreakHitResult` _outhit))
    (if (!= _hitactor (`self.LookAtActor`))
      (bind _output_get (set `self.LookAtActor` _hitactor))
      (message `/Game/MyContent/InventorySystem/BI_InteractInterface.LookAt` _output_get)
      (set `self.LookAtClass` (`GameplayStatics.GetObjectClass` _output_get)))
    (else
      (set `self.LookAtActor` null)
      (set `self.LookAtClass` null))))

(fn `RemoveFromInventory`
  (params (Index :type Integer) (IsConsumed :type Boolean) (`WholeStack?` :type Boolean) (Amount :type Integer))
  (locals (Local_Item :type Name) (LocalQuantity :type Integer))
  (bind _index (`local.Index`))
  (bind (_output_itemid _output_quantity) (break `/Game/MyContent/InventorySystem/ST_SlotStruct` (`|GetArrayItem` (`self.Content`) Index)))
  (bind (_output_itemid_2 _output_quantity_2) (break `/Game/MyContent/InventorySystem/ST_SlotStruct` (`|GetArrayItem` (`self.Content`) (`local.Index`))))
  (bind (_output_itemid_3 _output_quantity_3) (break `/Game/MyContent/InventorySystem/ST_SlotStruct` (`|GetArrayItem` (`self.Content`) _index)))
  (bind _returnvalue (- _output_quantity_3 (`local.Amount`)))
  (set `local.Local_Item` _output_itemid)
  (set `local.LocalQuantity` _output_quantity)
  (`|ExecutionSequence`
    (:`then_0`
      (if (or (`local.WholeStack?`) (<= _output_quantity_2 1))
        (`KismetArrayLibrary.Array_Set` (`self.Content`) (`local.Index`) (make `/Game/MyContent/InventorySystem/ST_SlotStruct` "None") :!label _label)
        (if (not (`local.IsConsumed`))
          (`self.DropItem` (`local.Local_Item`) (`local.LocalQuantity`)))
        (elif (<= _returnvalue 0)
          (goto _label)
          (else
            (`KismetArrayLibrary.Array_Set` (`self.Content`) _index (make `/Game/MyContent/InventorySystem/ST_SlotStruct` _output_itemid_3 _returnvalue))))))
    (:`then_1`
      (`self.Update`))))

(fn `TransferSlots`
  (params (SourceIndex :type Integer) (SourceInventory :type "/Game/MyContent/InventorySystem/BP_InventorySystem Object Reference") (DestinationIndex :type Integer))
  (locals (LocalSlotContent :type "/Game/MyContent/InventorySystem/ST_SlotStruct Structure"))
  (set `local.LocalSlotContent` (`|GetArrayItem` (`/Game/MyContent/InventorySystem/BP_InventorySystem.Content` SourceInventory) SourceIndex))
  (if (< DestinationIndex 0)
    _
    (elif (not (== (`.ItemID_3_93977A374DFEC8717DA67D8287A40F51` (break `/Game/MyContent/InventorySystem/ST_SlotStruct` (`local.LocalSlotContent`))) (`.ItemID_3_93977A374DFEC8717DA67D8287A40F51` (break `/Game/MyContent/InventorySystem/ST_SlotStruct` (`|GetArrayItem` (`self.Content`) (`local.DestinationIndex`))))))
      (`KismetArrayLibrary.Array_Set` (`/Game/MyContent/InventorySystem/BP_InventorySystem.Content` (`local.SourceInventory`)) (`local.SourceIndex`) (`|GetArrayItem` (`self.Content`) (`local.DestinationIndex`)))
      (`KismetArrayLibrary.Array_Set` (`self.Content`) (`local.DestinationIndex`) (`local.LocalSlotContent`))
      (`self.Update`)
      (`self.Update` (`local.SourceInventory`)))))